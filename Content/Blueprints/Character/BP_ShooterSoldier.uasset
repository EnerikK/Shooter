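; Player soldier character Blueprint that handles the sniper scope overlay, with a leftover debug test for the mantle animation.
; ShowSniperScopeWidget creates WBP_SniperScope on first use, caches it and adds it to the viewport.
; The same ScopeZoomIn animation plays forward to show the scope and in reverse to hide it, each with its own 2D zoom sound.
; DebugKey1 prints a message and plays the AM_TallMantle montage.
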(event EventBeginPlay)

(event Collision|EventActorBeginOverlap
  (params (OtherActor :type Actor%20Object%20Reference)))

(event EventTick
  (params (DeltaSeconds :type Float%20%28single-precision%29)))

(event EventShowSniperScopeWidget
  (params (bShowScope :type Boolean))
  (Utilities|IsValid (Variables|Default|GetSniperScopeWidget)
    (:Is%20Valid
      _)
    (:Is%20Not%20Valid
      (bind _returnvalue (UserInterface|CreateWidget "/Game/Blueprints/HUD/WBP_SniperScope.WBP_SniperScope_C"))
      (bind _output_get (Variables|Default|SetSniperScopeWidget _returnvalue))
      (UserInterface|Viewport|AddtoViewport _output_get 0)))
  (if bShowScope
    (Utilities|IsValid (Variables|Default|GetSniperScopeWidget)
      (:Is%20Valid
        (UserInterface|Animation|PlayAnimation (Variables|Default|GetSniperScopeWidget) (Variables|/Game/Blueprints/HUD/WBP_SniperScope.WBP_SniperScope_C|GetScopeZoomIn (Variables|Default|GetSniperScopeWidget)) 0.0 1 "Forward" 1.0 false)
        (Audio|PlaySound2D "/Game/Assets/MilitaryWeapSilver/Sound/SniperRifle/Wavs/SniperRifle_ZoomIn.SniperRifle_ZoomIn" 1.0 1.0 0.0 0 0)))
    (else
      (Utilities|IsValid (Variables|Default|GetSniperScopeWidget)
        (:Is%20Valid
          (UserInterface|Animation|PlayAnimation (Variables|Default|GetSniperScopeWidget) (Variables|/Game/Blueprints/HUD/WBP_SniperScope.WBP_SniperScope_C|GetScopeZoomIn (Variables|Default|GetSniperScopeWidget)) 0.0 1 "Reverse" 1.0 false)
          (Audio|PlaySound2D "/Game/Assets/MilitaryWeapSilver/Sound/SniperRifle/Wavs/SniperRifle_ZoomOut.SniperRifle_ZoomOut" 1.0 1.0 0.0 0 0))))))

(event Input|KeyboardEvents|DebugKey1
  (params (Key :type Key%20Structure :default "None") (ActionValue :type Input%20Action%20Value%20Structure))
  (:Pressed
    (Development|PrintString "Hello")
    (Animation|PlayAnimMontage self "/Game/Blueprints/Character/Animation/Soldier/Animations/Montages/AM_TallMantle.AM_TallMantle" 1.0 "None")))

(fn ConstructionScript)